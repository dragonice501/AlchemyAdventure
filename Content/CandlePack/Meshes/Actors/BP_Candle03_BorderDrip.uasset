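; Candle actor (variant 03, border drip) that can be lit or unlit, with a flickering light.
; SetEnabled, run from the construction script, toggles the light and flame particle visibility and swaps the mesh between lit and off materials.
; On BeginPlay, the CandleFlicker timeline drives SSSlight intensity between MinIntensity and MaxIntensity, regardless of the enabled state.
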(event EventBeginPlay
  (bind _intensity (Timeline|CandleFlicker Play)
    (:Update
      (Rendering|Components|Light|SetIntensity (Variables|Default|GetSSSlight) (Math|Float|Lerp (Variables|Default|GetMinIntensity) (Variables|Default|GetMaxIntensity) _intensity)))))

(fn ConstructionScript
  (CallFunction|SetEnabled (Variables|Default|GetEnabled)))

(fn SetEnabled
  (params (Enabled :type Boolean))
  (bind _sm_candle01 (Variables|Default|GetSM_Candle01))
  (bind _output_get (Variables|Default|SetEnabled Enabled))
  (Rendering|SetVisibility (Variables|Default|GetSSSlight) _output_get false)
  (Rendering|SetVisibility (Variables|Default|GetPS_CandleFlame) _output_get false)
  (if _output_get
    (Rendering|Material|SetMaterial _sm_candle01 0 "/Game/CandlePack/Materials/MI_Candles.MI_Candles")
    (else
      (Rendering|Material|SetMaterial _sm_candle01 0 "/Game/CandlePack/Materials/MI_Candles_OFF.MI_Candles_OFF"))))