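; Base weapon Blueprint that deals damage to enemies through a capsule hitbox, which starts with collision off.
; EnableCollision clears the HitEnemies list and switches the capsule to query-only collision, and DisableCollision turns it off again.
; Overlapping a BP_EnemyBase applies BaseDamage, with HitEnemies limiting each enemy to one hit per activation.
; The IsAlive check after damage has no follow-up logic.
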(event OnComponentBeginOverlap(Capsule)
  (params (OverlappedComponent :type Primitive%20Component%20Object%20Reference) (OtherActor :type Actor%20Object%20Reference) (OtherComp :type Primitive%20Component%20Object%20Reference) (OtherBodyIndex :type Integer) (bFromSweep :type Boolean) (SweepResult :type Hit%20Result%20Structure%20%28by%20ref%29))
  (bind _hitenemies (Variables|Default|GetHitEnemies))
  (bind _asbp_enemy_base (Utilities|Casting|CastToBP_EnemyBase OtherActor))
  (if (not (Utilities|Array|ContainsItem _hitenemies OtherActor))
    (Utilities|Array|Add _hitenemies OtherActor)
    (Default|TakeDamage _asbp_enemy_base (Variables|Default|GetBaseDamage))
    (bind _returnvalue (Default|IsAlive _asbp_enemy_base))
    (if (not _returnvalue)
      _)))

(event EventBeginPlay
  (Collision|SetCollisionEnabled (Variables|Default|GetCapsule) "NoCollision"))

(fn ConstructionScript)

(fn EnableCollision
  (Utilities|Array|Clear (Variables|Default|GetHitEnemies))
  (Collision|SetCollisionEnabled (Variables|Default|GetCapsule) "QueryOnly"))

(fn DisableCollision
  (Collision|SetCollisionEnabled (Variables|Default|GetCapsule) "NoCollision"))