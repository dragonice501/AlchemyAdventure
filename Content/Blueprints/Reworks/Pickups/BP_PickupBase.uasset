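; BP_PickupBase is a pickup base Blueprint that makes itself available to the player as an interactable while in range.
; When a BP_PlayerBase begins overlapping its Sphere component, it stores that player and registers itself through AddInteractable.
; When that stored player ends the overlap, it calls RemoveInteractable and clears the reference.
; The file holds no collection or interaction logic, and its construction script is empty.
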(event OnComponentBeginOverlap(Sphere)
  (params (OverlappedComponent :type Primitive%20Component%20Object%20Reference) (OtherActor :type Actor%20Object%20Reference) (OtherComp :type Primitive%20Component%20Object%20Reference) (OtherBodyIndex :type Integer) (bFromSweep :type Boolean) (SweepResult :type Hit%20Result%20Structure%20%28by%20ref%29))
  (bind _asbp_player_base (Utilities|Casting|CastToBP_PlayerBase OtherActor))
  (bind _output_get (Variables|Default|SetPlayerCharacter _asbp_player_base))
  (Default|AddInteractable _output_get self))

(event OnComponentEndOverlap(Sphere)
  (params (OverlappedComponent :type Primitive%20Component%20Object%20Reference) (OtherActor :type Actor%20Object%20Reference) (OtherComp :type Primitive%20Component%20Object%20Reference) (OtherBodyIndex :type Integer))
  (if (== OtherActor (Variables|Default|GetPlayerCharacter))
    (Default|RemoveInteractable (Variables|Default|GetPlayerCharacter) self)
    (Variables|Default|SetPlayerCharacter 0)))

(fn ConstructionScript)