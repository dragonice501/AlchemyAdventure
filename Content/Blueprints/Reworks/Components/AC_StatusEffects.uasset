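; AC_StatusEffects is a component that spawns and tracks status effect actors for an owning actor.
; AddStatusEffect spawns the given effect at the owner's transform, and for Attack-type effects stores it in AttackEffects, activates it and attaches it to the owner.
; EffectDamage is an unfinished stub: it loops over AttackEffects with an empty body and its return node is unreachable.
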(event EventBeginPlay)

(event EventTick
  (params (DeltaSeconds :type Float%20%28single-precision%29)))

(fn AddStatusEffect
  (params (StatusEffect :type BP%20Status%20Effect%20Base%20Class%20Reference) (Owner :type Actor%20Object%20Reference))
  (bind _returnvalue (Game|SpawnActorfromClass StatusEffect (Transformation|GetActorTransform Owner) "Undefined" "MultiplyWithRoot" Owner 0))
  (switch Utilities|FlowControl|Switch|SwitchonE_EffectType (Variables|/Game/Blueprints/Reworks/StatusEffects/BP_StatusEffectBase.BP_StatusEffectBase_C|GetEffectType _returnvalue)
    (:NewEnumerator1
      (Utilities|Array|Add (Variables|Default|GetAttackEffects) _returnvalue)
      (Default|Activate _returnvalue)
      (Transformation|AttachActorToActor _returnvalue Owner "None" "KeepRelative" "KeepRelative" "KeepRelative" true))))

(fn EffectDamage
  (params (BaseDamage :type Float%20%28double-precision%29))
  (for _array_element (Variables|Default|GetAttackEffects)
    _))