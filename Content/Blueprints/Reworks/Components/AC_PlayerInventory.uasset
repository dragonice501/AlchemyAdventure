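; Player inventory component that stores weapons in an array and stacks resources and usables in maps of item to count.
; Index-based getters use map key order to return items, images and counts, while adds return the slot index.
; Crafting checks the first resource's two combinable names against the second and fetches the result from the Craftables data table, which also supplies added usables.
; Resources are decremented by index, and a separate pass removes depleted entries using an index offset.
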(event EventBeginPlay)

(event EventTick
  (params (DeltaSeconds :type Float%20%28single-precision%29)))

(fn AddResource
  (params (Resource :type S%20Resource%20Structure))
  (bind _resources (Variables|Default|GetResources))
  (bind _keys (Utilities|Map|Keys (Variables|Default|GetResources)))
  (if (!= (Utilities|Array|FindItem _keys Resource) -1)
    (bind _result (Math|Integer|IncrementInt (.Value (Utilities|Map|Find _resources Resource)))
      (:%20%20
        (Utilities|Map|Add _resources Resource _result)
        (return (Utilities|Array|FindItem _keys Resource) _result)))
    (else
      (Utilities|Map|Add (Variables|Default|GetResources) Resource 1)
      (bind _keys_2 (Utilities|Map|Keys (Variables|Default|GetResources)))
      (return (Utilities|Array|FindItem _keys_2 Resource) 1))))

(fn AddWeapon
  (params (Weapon :type S%20Weapon%20Structure))
  (bind _returnvalue (Utilities|Array|Add (Variables|Default|GetWeapons) Weapon))
  (return _returnvalue))

(fn GetResourceImageatIndex
  (params (Index :type Integer))
  (bind _keys (Utilities|Map|Keys (Variables|Default|GetResources)))
  (if (< Index (Utilities|Array|Length _keys))
    (return (.resourceimage (Utilities|Array|Get(acopy) _keys Index)))
    (else
      (return 0))))

(fn GetWeaponImageatIndex
  (params (Index :type Integer))
  (bind _weapons (Variables|Default|GetWeapons))
  (if (< Index (Utilities|Array|Length _weapons))
    (return (.weaponimage (Utilities|Array|Get(acopy) _weapons Index)))
    (else
      (return 0))))

(fn GetResourceatIndex
  (params (Index :type Integer))
  (bind _keys (Utilities|Map|Keys (Variables|Default|GetResources)))
  (if (< Index (Utilities|Array|Length _keys))
    (return (Utilities|Array|Get(acopy) _keys Index))
    (else
      (return ""))))

(fn GetWeaponatIndex
  (params (Index :type Integer))
  (bind _weapons (Variables|Default|GetWeapons))
  (if (< Index (Utilities|Array|Length _weapons))
    (return (Utilities|Array|Get(acopy) _weapons Index))
    (else
      (return ""))))

(fn GetCraftable
  (params (IndexOne :type Integer) (IndexTwo :type Integer))
  (bind _keys (Utilities|Map|Keys (Variables|Default|GetResources)))
  (bind _output_get (LocalVariables|SetResources _keys))
  (if (Utilities|Enum|Equal(Enum) (.combinableone (Utilities|Array|Get(acopy) _output_get IndexOne)) (.name (Utilities|Array|Get(acopy) (LocalVariables|GetResources) IndexTwo)))
    (bind _returnvalue (Utilities|GetDataTableRow (Variables|Default|GetCraftables) (Utilities|String|StringToName (.combineresultone (Utilities|Array|Get(acopy) _output_get IndexOne))))
      (:then
        (return _returnvalue)))
    (elif (Utilities|Enum|Equal(Enum) (.combinabletwo (Utilities|Array|Get(acopy) _output_get IndexOne)) (.name (Utilities|Array|Get(acopy) (LocalVariables|GetResources) IndexTwo)))
      (bind _returnvalue_2 (Utilities|GetDataTableRow (Variables|Default|GetCraftables) (Utilities|String|StringToName (.combineresulttwo (Utilities|Array|Get(acopy) _output_get IndexOne))))
        (:then
          (return _returnvalue_2)))
      (else
        (return "")))))

(fn AddUsable
  (params (Usable :type String))
  (bind _usables (Variables|Default|GetUsables))
  (bind _returnvalue (Utilities|GetDataTableRow (Variables|Default|GetCraftables) (Utilities|String|StringToName Usable))
    (:then
      (LocalVariables|SetNewUsable _returnvalue)
      (bind _keys (Utilities|Map|Keys (Variables|Default|GetUsables)))
      (if (!= (Utilities|Array|FindItem _keys (LocalVariables|GetNewUsable)) -1)
        (bind _result (Math|Integer|IncrementInt (.Value (Utilities|Map|Find _usables (LocalVariables|GetNewUsable))))
          (:%20%20
            (Utilities|Map|Add _usables (LocalVariables|GetNewUsable) _result)
            (return (Utilities|Array|FindItem _keys (LocalVariables|GetNewUsable)) (LocalVariables|GetNewUsable) _result)))
        (else
          (Utilities|Map|Add (Variables|Default|GetUsables) (LocalVariables|GetNewUsable) 1)
          (bind _keys_2 (Utilities|Map|Keys (Variables|Default|GetUsables)))
          (return (Utilities|Array|FindItem _keys_2 (LocalVariables|GetNewUsable)) (LocalVariables|GetNewUsable) 1))))))

(fn GetUsableatIndex
  (params (Index :type Integer))
  (bind _keys (Utilities|Map|Keys (Variables|Default|GetUsables)))
  (if (< Index (Utilities|Array|Length _keys))
    (return (Utilities|Array|Get(acopy) _keys Index))
    (else
      (return ""))))

(fn DecrementResourceatIndex
  (params (Index :type Integer))
  (bind _resources (Variables|Default|GetResources))
  (bind _keys (Utilities|Map|Keys _resources))
  (bind _result (Math|Integer|DecrementInt (.Value (Utilities|Map|Find _resources (Utilities|Array|Get(acopy) _keys Index))))
    (:%20%20
      (Utilities|Map|Add _resources (Utilities|Array|Get(acopy) _keys Index) _result))))

(fn UpdateResources
  (bind _resources (Variables|Default|GetResources))
  (bind _values (Utilities|Map|Values _resources))
  (for (_array_element _array_index) _values
    (if (<= _array_element 0)
      (bind _keys (Utilities|Map|Keys _resources))
      (Utilities|Map|Remove _resources (Utilities|Array|Get(acopy) _keys (- _array_index (LocalVariables|GetIndexOffset))))
      (bind _result (Math|Integer|IncrementInt (LocalVariables|GetIndexOffset))
        (:%20%20
          (LocalVariables|SetIndexOffset _result))))))

(fn GetResourceImageandCount
  (params (Index :type Integer))
  (bind _resources (Variables|Default|GetResources))
  (bind _keys (Utilities|Map|Keys _resources))
  (if (< Index (Utilities|Array|Length _keys))
    (bind _values (Utilities|Map|Values _resources))
    (return (.resourceimage (Utilities|Array|Get(acopy) _keys Index)) (Utilities|Array|Get(acopy) _values Index))
    (else
      (return 0 0))))

(fn HasResourceatIndex
  (params (Index :type Integer))
  (return (> (Utilities|Map|Length (Variables|Default|GetResources)) Index)))

(fn GetUsableandCountatIndex
  (params (Index :type Integer))
  (bind _usables (Variables|Default|GetUsables))
  (bind _keys (Utilities|Map|Keys _usables))
  (if (< Index (Utilities|Array|Length _keys))
    (bind _values (Utilities|Map|Values _usables))
    (return (.image (Utilities|Array|Get(acopy) _keys Index)) (Utilities|Array|Get(acopy) _values Index))
    (else
      (return 0 0))))