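; Base player character handling interactables, inventory, right-hand weapons and enemy lock-on.
; Lock-on targets the first tracked enemy; a timeline blends camera and control rotation toward it, with the camera aimed at the player-to-target midpoint.
; The interactable most aligned with the actor's forward vector becomes current.
; ACPlayerInventory additions update HUD icons, and three shortcut inputs toggle equipment slots, spawning weapons attached to a mesh socket.
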(event Custom|StartCameraLookAtEnemy
  (Variables|Camera|SetCameraLerping true)
  (bind (_direction _delta) (Timeline|Timeline PlayFromStart)
    (:Update
      (switch Utilities|FlowControl|Switch|SwitchonETimelineDirection _direction
        (:Forward
          (CallFunction|LerpCameratoCombatTarget _delta))
        (:Backward
          (Transformation|SetRelativeRotation (Variables|Default|GetCamera) "0, 0, 0" false false))))
    (:Finished
      (Variables|Camera|SetCameraLerping false))))

(event Custom|EndCameraLookAtEnemy
  (Transformation|SetRelativeRotation (Variables|Default|GetCamera) "0, 0, 0" false false))

(event Input|EnhancedActionEvents|EnhancedInputActionIA_OneShortcut
  (params (ActionValue :type Boolean) (ElapsedSeconds :type Float%20%28double-precision%29) (TriggeredSeconds :type Float%20%28double-precision%29) (InputAction :type Input%20Action%20Object%20Reference :default "/Game/Input/IA_OneShortcut.IA_OneShortcut"))
  (CallFunction|SetWeaponRight))

(event Input|EnhancedActionEvents|EnhancedInputActionIA_TwoShortcut
  (params (ActionValue :type Boolean) (ElapsedSeconds :type Float%20%28double-precision%29) (TriggeredSeconds :type Float%20%28double-precision%29) (InputAction :type Input%20Action%20Object%20Reference :default "/Game/Input/IA_TwoShortcut.IA_TwoShortcut"))
  (CallFunction|SetWeaponRight 1))

(event Input|EnhancedActionEvents|EnhancedInputActionIA_ThreeShortcut
  (params (ActionValue :type Boolean) (ElapsedSeconds :type Float%20%28double-precision%29) (TriggeredSeconds :type Float%20%28double-precision%29) (InputAction :type Input%20Action%20Object%20Reference :default "/Game/Input/IA_ThreeShortcut.IA_ThreeShortcut"))
  (CallFunction|SetWeaponRight 2))

(event EventBeginPlay
  (|CallParentFunction) ; This node is disabled and will not be called.\nDrag off pins to build functionality.
)

(event Collision|EventActorBeginOverlap
  (params (OtherActor :type Actor%20Object%20Reference))
  (|CallParentFunction OtherActor) ; This node is disabled and will not be called.\nDrag off pins to build functionality.
)

(event EventTick
  (params (DeltaSeconds :type Float%20%28single-precision%29))
  (|CallParentFunction DeltaSeconds) ; This node is disabled and will not be called.\nDrag off pins to build functionality.
)

(fn ConstructionScript
  (|CallParentFunction))

(fn AddInteractable
  (params (Interactable :type Actor%20Object%20Reference))
  (Utilities|Array|Add (Variables|Interaction|GetInteractables) Interactable)
  (Interaction|SetInteractable))

(fn AddResource
  (params (Resource :type S%20Resource%20Structure))
  (bind _returnvalue (Default|AddResource (Variables|Default|GetAC_PlayerInventory) Resource))
  (bind _keys (Utilities|Map|Keys (Variables|/Game/Blueprints/Reworks/Components/AC_PlayerInventory.AC_PlayerInventory_C|GetResources (Variables|Default|GetAC_PlayerInventory))))
  (Utilities|IsValid (.resourceimage (Utilities|Array|Get(acopy) _keys _returnvalue))
    (:Is%20Valid
      (Default|UpdateResourceInventoryatIndex (Variables|Default|GetHUD) _returnvalue (.resourceimage (Utilities|Array|Get(acopy) _keys _returnvalue))))))

(fn RemoveInteractable
  (params (Interactable :type Actor%20Object%20Reference))
  (Utilities|Array|RemoveItem (Variables|Interaction|GetInteractables) Interactable)
  (Interaction|SetInteractable))

(fn GetMostForwardInteractable
  (bind _interactables (Variables|Interaction|GetInteractables))
  (bind _interactables_2 (Variables|Interaction|GetInteractables))
  (Utilities|FlowControl|Sequence
    (:then_0
      (if (== (Utilities|Array|Length (Variables|Interaction|GetInteractables)) 0)
        (return 0)))
    (:then_1
      (if (== (Utilities|Array|Length _interactables_2) 1)
        (return (Utilities|Array|Get(acopy) _interactables_2))))
    (:then_2
      (if (> (Utilities|Array|Length _interactables) 1)
        (LocalVariables|SetSmallestDot 1e+04)
        (LocalVariables|SetClosestIndex 0)
        (for (_array_element _array_index) _interactables
          (if (< (- 1.0 (Math|Vector|DotProduct (Transformation|GetActorForwardVector) (Math|Vector|Normalize (- (Transformation|GetActorLocation _array_element) (Transformation|GetActorLocation))))) (LocalVariables|GetSmallestDot))
            (LocalVariables|SetSmallestDot (- 1.0 (Math|Vector|DotProduct (Transformation|GetActorForwardVector) (Math|Vector|Normalize (- (Transformation|GetActorLocation _array_element) (Transformation|GetActorLocation))))))
            (LocalVariables|SetClosestIndex _array_index)))
        (return (Utilities|Array|Get(acopy) (Variables|Interaction|GetInteractables) (LocalVariables|GetClosestIndex)))))))

(fn SetInteractable
  (bind _interactable (Interaction|GetMostForwardInteractable))
  (Variables|Interaction|SetInteractable _interactable))

(fn AddWeapon
  (params (Weapon :type S%20Weapon%20Structure))
  (bind _ac_playerinventory (Variables|Default|GetAC_PlayerInventory))
  (bind _returnvalue (Default|AddWeapon _ac_playerinventory Weapon))
  (Utilities|IsValid (.weaponimage (Utilities|Array|Get(acopy) (Variables|/Game/Blueprints/Reworks/Components/AC_PlayerInventory.AC_PlayerInventory_C|GetWeapons _ac_playerinventory) _returnvalue))
    (:Is%20Valid
      (Default|UpdateWeaponInventoriesatIndex (Variables|Default|GetHUD) _returnvalue (.weaponimage (Utilities|Array|Get(acopy) (Variables|/Game/Blueprints/Reworks/Components/AC_PlayerInventory.AC_PlayerInventory_C|GetWeapons _ac_playerinventory) _returnvalue))))))

(fn AddEnemy
  (params (Enemy :type BP%20Enemy%20Base%20Object%20Reference))
  (Utilities|Array|Add (Variables|Combat|GetEnemies) Enemy))

(fn RemoveEnemy
  (params (Enemy :type BP%20Enemy%20Base%20Object%20Reference))
  (Utilities|Array|RemoveItem (Variables|Combat|GetEnemies) Enemy))

(fn UnlockonEnemy
  (Default|SetHealthBarVisibility (Variables|Combat|GetTargetEnemy) false)
  (Variables|Combat|SetTargetEnemy 0)
  (Default|SetTargetLock (Variables|Default|GetHUD) false)
  (Variables|/Script/Engine.CharacterMovementComponent|SetbOrientRotationToMovement (Variables|Character|GetCharacterMovement) true)
  (Variables|Combat|SetLockedOn false)
  (Variables|Camera|SetCameraCurrentRotation (Variables|/Script/Engine.SceneComponent|GetRelativeRotation (Variables|Default|GetCamera))))

(fn GetCameraTargetLookat
  (bind _returnvalue (Transformation|GetActorLocation))
  (bind _targetenemy (Variables|Combat|GetTargetEnemy)
    (:then
      (return (Math|Rotator|FindLookatRotation (Transformation|GetWorldLocation (Variables|Default|GetCamera)) (+ _returnvalue (/ (- (Default|GetLockonLocation _targetenemy) _returnvalue) 2.0)))))
    (:else)))

(fn GetCombatTargetLookat
  (bind _targetenemy (Variables|Combat|GetTargetEnemy)
    (:then
      (return (Math|Rotator|MakeRotator 0.0 (Variables|Camera|GetCombatCameraPitch) (.yaw (Math|Rotator|FindLookatRotation (Transformation|GetActorLocation) (Transformation|GetActorLocation _targetenemy))))))
    (:else)))

(fn LerpCameratoCombatTarget
  (params (Delta :type Float%20%28double-precision%29))
  (Transformation|SetWorldRotation (Variables|Default|GetCamera) (Math|Rotator|Lerp(Rotator) (Variables|Camera|GetCameraCurrentRotation) (Combat|GetCameraTargetLookat) Delta true) false false)
  (Pawn|SetControlRotation (Variables|Default|GetControllerBase) (Math|Rotator|Lerp(Rotator) (Variables|Camera|GetCameraBoomStartRotation) (CallFunction|GetCombatTargetLookat) Delta true)))

(fn LookatCombatTarget
  (Transformation|SetActorRotation (Math|Rotator|MakeRotator 0.0 0.0 (.yaw (Math|Rotator|FindLookatRotation (Transformation|GetActorLocation) (Transformation|GetActorLocation (Variables|Combat|GetTargetEnemy))))))
  (if (not (Variables|Camera|GetCameraLerping))
    (Transformation|SetWorldRotation (Variables|Default|GetCamera) (Combat|GetCameraTargetLookat) false false)
    (Pawn|SetControlRotation (Variables|Default|GetControllerBase) (CallFunction|GetCombatTargetLookat))))

(fn LockonEnemy
  (bind _enemies (Variables|Combat|GetEnemies))
  (if (> (Utilities|Array|Length _enemies) 0)
    (bind _output_get (Variables|Combat|SetTargetEnemy (Utilities|Array|Get(acopy) _enemies)))
    (Default|SetHealthBarVisibility _output_get true)
    (Default|SetTargetLock (Variables|Default|GetHUD) true)
    (Variables|/Script/Engine.CharacterMovementComponent|SetbOrientRotationToMovement (Variables|Character|GetCharacterMovement) false)
    (Variables|Combat|SetLockedOn true)
    (Variables|Camera|SetCameraCurrentRotation (Transformation|GetWorldRotation (Variables|Default|GetCamera)))
    (Variables|Camera|SetCameraBoomStartRotation (Pawn|GetControlRotation :!class /Script/Engine.Pawn))))

(fn SetWeaponRight
  (params (WeaponIndex :type Integer))
  (if (== (Variables|Equipment|GetWeaponRightIndexCurrent) WeaponIndex)
    (CallFunction|RemoveRightWeapon)
    (Variables|Equipment|SetWeaponRightIndexCurrent -1)
    (Variables|Equipment|SetRightEquipped false)
    (return false)
    (else
      (CallFunction|EquipRightWeapon WeaponIndex))))

(fn RemoveRightWeapon
  (Variables|Equipment|GetWeaponRight
    (:then
      (Actor|DestroyActor (Variables|Equipment|GetWeaponRight))
      (Variables|Equipment|SetWeaponRight 0))
    (:else)))

(fn SetRightEquipmentatIndex
  (params (InventoryIndex :type Integer) (EquipmentIndex :type Integer))
  (bind _weaponrightindexcurrent (Variables|Equipment|GetWeaponRightIndexCurrent))
  ;[0 0 0] Remove weapon if already in use
  (for (_array_element _array_index) (Variables|Equipment|GetWeaponRightIndeces)
    (if (== _array_element InventoryIndex)
      (Utilities|Array|SetArrayElem (Variables|Equipment|GetWeaponRightIndeces) _array_index -1)
      (Utilities|Array|SetArrayElem (Variables|Equipment|GetWeaponsRight) _array_index 0)
      (Default|UpdateWeaponSelectInvatIndex (Variables|Default|GetHUD) _array_index)))
  (Utilities|Array|SetArrayElem (Variables|Equipment|GetWeaponsRight) EquipmentIndex (.weapon (Utilities|Array|Get(acopy) (Variables|/Game/Blueprints/Reworks/Components/AC_PlayerInventory.AC_PlayerInventory_C|GetWeapons (Variables|Default|GetAC_PlayerInventory)) InventoryIndex)))
  (Utilities|Array|SetArrayElem (Variables|Equipment|GetWeaponRightIndeces) EquipmentIndex InventoryIndex)
  (if (== EquipmentIndex _weaponrightindexcurrent)
    (CallFunction|RemoveRightWeapon)
    (CallFunction|EquipRightWeapon _weaponrightindexcurrent)))

(fn EquipRightWeapon
  (params (EquipmentIndex :type Integer))
  (bind _weaponsright (Variables|Equipment|GetWeaponsRight))
  (bind _output (Utilities|Array|Get(acopy) _weaponsright EquipmentIndex))
  (if (Utilities|IsValidClass _output)
    (Variables|Equipment|SetWeaponRightIndexCurrent EquipmentIndex)
    (bind _asbp_weapon_base (Utilities|Casting|CastToBP_WeaponBaseClass _output))
    (CallFunction|RemoveRightWeapon)
    (bind _returnvalue (Game|SpawnActorfromClass _asbp_weapon_base (Transformation|GetSocketTransform (Variables|Character|GetMesh) (Variables|Equipment|GetWeaponRightSocket) "RTS_World") "Undefined" "MultiplyWithRoot" 0 0))
    (bind _output_get (Variables|Equipment|SetWeaponRight _returnvalue))
    (Variables|/Game/Blueprints/Reworks/Equipment/BP_WeaponBase.BP_WeaponBase_C|SetOwningCharacter _output_get self)
    (bind _returnvalue_2 (Transformation|AttachComponentToComponent _output_get (Variables|Character|GetMesh) (Variables|Equipment|GetWeaponRightSocket) "SnapToTarget" "SnapToTarget" "SnapToTarget" true))
    (bind _output_get_2 (Variables|Equipment|SetRightEquipped _returnvalue_2))
    (return _output_get_2)))