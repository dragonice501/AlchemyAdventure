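; BP_CharacterBase is a character base Blueprint that provides simple health and death logic.
; TakeDamage subtracts damage from Health, clamps the result between zero and MaxHealth, and calls Die whenever Health is at zero afterward.
; IsAlive reports whether Health is above zero.
; Die is an empty stub, and BeginPlay, Tick, overlap and the construction script contain no logic.
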(event EventBeginPlay)

(event Collision|EventActorBeginOverlap
  (params (OtherActor :type Actor%20Object%20Reference)))

(event EventTick
  (params (DeltaSeconds :type Float%20%28single-precision%29)))

(fn ConstructionScript)

(fn TakeDamage
  (params (Damage :type Float%20%28double-precision%29))
  (bind _output_get (Variables|Attributes|SetHealth (Math|Float|Clamp(Float) (- (Variables|Attributes|GetHealth) Damage) 0.0 (Variables|Attributes|GetMaxHealth))))
  (if (<= _output_get 0.0)
    (CallFunction|Die)))

(fn IsAlive
  (return (> (Variables|Attributes|GetHealth) 0.0)))

(fn Die)