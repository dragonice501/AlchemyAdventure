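; Player character Blueprint that handles Enhanced Input movement, camera look, interaction, menu toggling and melee combat.
; It creates the HUD overlay and drives its interact prompt, menu and lock-on marker, while feeding movement input to the AnimInstance.
; Attacks play combo-numbered montage sections, with events toggling weapon collision and reopening the combo.
; When not locked on, a timeline turns the character toward camera-relative input as attack collision starts.
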(event Custom|SetInteractWidget
  (bind _hud (Variables|Default|GetHUD))
  (if (and (Utilities|IsValid (Variables|Default|GetInteractable)) (not (Variables|Default|GetMenuing)))
    (Default|SetInteractWidget _hud true)
    (else
      (Default|SetInteractWidget _hud false))))

(event Custom|RotateTowardsAttackInput
  ;[1 1 1] Movement
  (if (> (Class|KismetMathLibrary|VSize2DSquared (Input|EnhancedActionValues|GetIA_Move)) 0.0)
    (bind _output_get (Variables|Combat|SetAttackStartRotation (Transformation|GetActorRotation)))
    (bind _delta (Timeline|AttackInputRotate PlayFromStart)
      (:Update
        (Transformation|SetActorRotation (Math|Rotator|Lerp(Rotator) _output_get (CallFunction|GetAttackInputRotation) _delta true))))))

(event Input|EnhancedActionEvents|EnhancedInputActionIA_Move
  (params (ActionValue :type Vector%202D%20Structure) (ElapsedSeconds :type Float%20%28double-precision%29) (TriggeredSeconds :type Float%20%28double-precision%29) (InputAction :type Input%20Action%20Object%20Reference :default "/Game/Input/IA_Move.IA_Move"))
  ;[1 1 1] Movement
  (CallFunction|Move (.x ActionValue) (.y ActionValue))
  (if (> (Utilities|Array|Length (Variables|Default|GetInteractables)) 0)
    (CallFunction|SetInteractable)))

(event Input|EnhancedActionEvents|EnhancedInputActionIA_Look
  (params (ActionValue :type Vector%202D%20Structure) (ElapsedSeconds :type Float%20%28double-precision%29) (TriggeredSeconds :type Float%20%28double-precision%29) (InputAction :type Input%20Action%20Object%20Reference :default "/Game/Input/IA_Look.IA_Look"))
  (if (not (Variables|Default|GetCameraLerping))
    (Pawn|Input|AddControllerYawInput (.x ActionValue))
    (Pawn|Input|AddControllerPitchInput (.y ActionValue))))

(event Input|EnhancedActionEvents|EnhancedInputActionIA_Interact
  (params (ActionValue :type Boolean) (ElapsedSeconds :type Float%20%28double-precision%29) (TriggeredSeconds :type Float%20%28double-precision%29) (InputAction :type Input%20Action%20Object%20Reference :default "/Game/Input/IA_Interact.IA_Interact"))
  (:Started
    (if (and (Utilities|IsValid (Variables|Default|GetInteractable)) (not (Variables|Default|GetMenuing)))
      (Class|BPIInteractable|Interact(Message) (Variables|Default|GetInteractable))
      (CallFunction|SetInteractable))))

(event Input|EnhancedActionEvents|EnhancedInputActionIA_ToggleLockOn
  (params (ActionValue :type Boolean) (ElapsedSeconds :type Float%20%28double-precision%29) (TriggeredSeconds :type Float%20%28double-precision%29) (InputAction :type Input%20Action%20Object%20Reference :default "/Game/Input/IA_ToggleLockOn.IA_ToggleLockOn"))
  (:Started
    (if (Variables|Default|GetLockedOn)
      (CallFunction|UnlockonEnemy)
      (Variables|Default|GetTargetEnemy
        (:then
          (CallFunction|EndCameraLookatEnemy))
        (:else))
      (else
        (CallFunction|LockonEnemy)
        (Variables|Default|GetTargetEnemy
          (:then
            (CallFunction|StartCameraLookatEnemy))
          (:else))))))

(event Input|EnhancedActionEvents|EnhancedInputActionIA_Attack
  (params (ActionValue :type Boolean) (ElapsedSeconds :type Float%20%28double-precision%29) (TriggeredSeconds :type Float%20%28double-precision%29) (InputAction :type Input%20Action%20Object%20Reference :default "/Game/Input/IA_Attack.IA_Attack"))
  (:Started
    (Variables|Default|GetWeaponRight
      (:then
        (if (Variables|Combat|GetCanAttack)
          (Animation|PlayAnimMontage (Variables|Default|GetAttackMontage) 1.0 (Utilities|String|StringToName (Utilities|String|Append (Variables|Default|GetAttackMontageSection) (Utilities|String|ToString(Integer) (Variables|Combat|GetComboCount)))))
          (Variables|Combat|SetCanAttack false)))
      (:else))))

(event Input|EnhancedActionEvents|EnhancedInputActionIA_Menu
  (params (ActionValue :type Boolean) (ElapsedSeconds :type Float%20%28double-precision%29) (TriggeredSeconds :type Float%20%28double-precision%29) (InputAction :type Input%20Action%20Object%20Reference :default "/Game/Input/IA_Menu.IA_Menu"))
  (CallFunction|HandleMenu))

(event EventBeginPlay
  (CallFunction|SetupIMC)
  (CallFunction|SetupHUD)
  (Variables|Default|SetAnimInstance (Components|SkeletalMesh|GetAnimInstance (Variables|Character|GetMesh))))

(event EventResetAttacking
  (Variables|Combat|SetCanAttack true)
  (Variables|Combat|SetComboCount 1))

(event EventTick
  (params (DeltaSeconds :type Float%20%28single-precision%29))
  (bind _returnvalue (Input|EnhancedActionValues|GetIA_Move))
  (Class|BPIAnimation|SetDirectionInputs(Message) (Variables|Default|GetAnimInstance) (.x _returnvalue) (.y _returnvalue))
  (if (Variables|Default|GetLockedOn)
    (CallFunction|LookatCombatTarget)
    (bind _targetenemy (Variables|Default|GetTargetEnemy)
      (:then
        (Default|SetTargetLockLocation (Variables|Default|GetHUD) (Default|GetLockonLocation _targetenemy)))
      (:else))))

(event EventOpenCombo
  (Math|Integer|IncrementInt (Variables|Combat|GetComboCount)
    (:%20%20
      (Variables|Combat|SetCanAttack true))))

(event EventStartAttackCollision
  (bind _weaponright (Variables|Default|GetWeaponRight)
    (:then
      (Default|EnableCollision _weaponright)
      (if (not (Variables|Default|GetLockedOn))
        (CallFunction|RotateTowardsAttackInput)))
    (:else)))

(event EventEndAttackCollision
  (bind _weaponright (Variables|Default|GetWeaponRight)
    (:then
      (Default|DisableCollision _weaponright)
      (Variables|Combat|SetAttacking false))
    (:else)))

(fn ConstructionScript
  (|CallParentFunction))

(fn AddInteractable
  (params (Interactable :type Actor%20Object%20Reference))
  (|CallParentFunction Interactable)
  (CallFunction|SetInteractWidget))

(fn RemoveInteractable
  (params (Interactable :type Actor%20Object%20Reference))
  (|CallParentFunction Interactable)
  (CallFunction|SetInteractWidget))

(fn SetupIMC
  (bind _asbp_controller_base (Utilities|Casting|CastToBP_ControllerBase (Pawn|GetController)))
  (bind _output_get (Variables|Default|SetControllerBase _asbp_controller_base))
  (Input|AddMappingContext (PlayerController|LocalPlayerSubsystems|GetEnhancedInputLocalPlayerSubsystem _output_get) "/Game/Input/IMC_PlayerCharacter.IMC_PlayerCharacter" 0 "(bIgnoreAllPressedKeysUntilRelease=True,bForceImmediately=False,bNotifyUserSettings=False)"))

(fn SetupHUD
  (bind _returnvalue (UserInterface|CreateWidget "/Game/Blueprints/Reworks/UI/WBP_HUDOverlay.WBP_HUDOverlay_C"))
  (bind _output_get (Variables|Default|SetHUD _returnvalue))
  (UserInterface|Viewport|AddtoViewport _output_get 0)
  (CallFunction|SetInteractWidget))

(fn Move
  (params (X :type Float%20%28single-precision%29) (Y :type Float%20%28single-precision%29))
  (bind _controllerbase (Variables|Default|GetControllerBase))
  (bind _returnvalue (Pawn|GetControlRotation _controllerbase :!class /Script/Engine.Controller))
  (Pawn|Input|AddMovementInput (Math|Vector|GetForwardVector _returnvalue) Y false)
  (Pawn|Input|AddMovementInput (Math|Vector|GetRightVector _returnvalue) X false))

(fn AdjustControlRotation
  (bind _returnvalue (Pawn|GetControlRotation :!class /Script/Engine.Pawn))
  (if (< (.pitch _returnvalue) 0.0)
    (Pawn|Input|AddControllerPitchInput 3.6e+02)
    (if (< (.yaw _returnvalue) 0.0)
      (Pawn|Input|AddControllerYawInput 3.6e+02))))

(fn GetAttackInputRotation
  (bind _returnvalue (Input|EnhancedActionValues|GetIA_Move))
  (return (Math|Rotator|MakeRotator 0.0 0.0 (- (.yaw (Pawn|GetControlRotation (Variables|Default|GetControllerBase) :!class /Script/Engine.Controller)) (- (.yaw (Math|Rotator|MakeRotfromX (Math|Vector|MakeVector (.x _returnvalue) (.y _returnvalue) 0.0))) 9e+01)))))

(fn HandleMenu
  (bind _controllerbase (Variables|Default|GetControllerBase))
  (bind _hud (Variables|Default|GetHUD))
  (bind _hud_2 (Variables|Default|GetHUD))
  (Variables|Default|GetHUD
    (:then
      (bind _output_get (Variables|Default|SetMenuing (not (Variables|Default|GetMenuing))))
      (if _output_get
        (Default|SetMainMenu _hud true)
        (Default|SetInteractWidget _hud false)
        (Input|SetInputModeGameandUI (Variables|Default|GetControllerBase) 0 "LockInFullscreen" false false)
        (Variables|/Script/Engine.PlayerController|SetbShowMouseCursor (Variables|Default|GetControllerBase) true)
        (else
          (Default|SetMainMenu _hud_2 false)
          (Default|HideMenus _hud_2)
          (Variables|Default|GetInteractable
            (:then
              (Default|SetInteractWidget _hud_2 false))
            (:else
              _))
          (Input|SetInputModeGameOnly _controllerbase false)
          (Variables|/Script/Engine.PlayerController|SetbShowMouseCursor _controllerbase false))))
    (:else)))