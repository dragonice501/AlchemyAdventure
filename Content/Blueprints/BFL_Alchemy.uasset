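; BFL_Alchemy is a Blueprint function library with a damage formula for combat between characters.
; CalculateDamage adds the attacker's augmented Might, attack chain bonus and the weapon damage.
; It then scales that sum by the target's physical resistance, treated as a percentage reduction.
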(fn CalculateDamage
  (params (Attacker :type BP%20Character%20Base%20Object%20Reference) (Target :type BP%20Character%20Base%20Object%20Reference) (WeaponDamage :type Float%20%28double-precision%29))
  (bind _ac_characterattributes (Variables|/Game/Blueprints/Characters/BP_CharacterBase.BP_CharacterBase_C|GetAC_CharacterAttributes Attacker))
  (return (* (+ (+ (.augmented (Variables|/Game/Blueprints/Components/AC_AttributesBase.AC_AttributesBase_C|GetMightC _ac_characterattributes)) (Variables|/Game/Blueprints/Components/AC_CharacterAttributes.AC_CharacterAttributes_C|GetAttackChainBonus _ac_characterattributes)) WeaponDamage) (Math|Float|SafeDivide (- 1e+02 (Variables|/Game/Blueprints/Components/AC_CharacterAttributes.AC_CharacterAttributes_C|GetPhysicalResistance (Variables|/Game/Blueprints/Characters/BP_CharacterBase.BP_CharacterBase_C|GetAC_CharacterAttributes Target))) 1e+02))))