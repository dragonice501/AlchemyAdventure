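; BP_StatusEffectHeal is a status effect that heals the character that owns it.
; It overrides Activate, calling the parent version, then casting its owner to BP_CharacterBase and calling Heal with EffectModifier truncated to an integer.
; The event graph holds only disabled default nodes, so all of its own logic runs on activation.
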(event EventBeginPlay
  (|CallParentFunction) ; This node is disabled and will not be called.\nDrag off pins to build functionality.
)

(event Collision|EventActorBeginOverlap
  (params (OtherActor :type Actor%20Object%20Reference))
  (|CallParentFunction OtherActor) ; This node is disabled and will not be called.\nDrag off pins to build functionality.
)

(event EventTick
  (params (DeltaSeconds :type Float%20%28single-precision%29)))

(fn ConstructionScript
  (|CallParentFunction))

(fn Activate
  (|CallParentFunction)
  (bind _asbp_character_base (Utilities|Casting|CastToBP_CharacterBase (Components|GetOwner)))
  (Default|Heal _asbp_character_base (Math|Float|Truncate (Variables|Default|GetEffectModifier))))