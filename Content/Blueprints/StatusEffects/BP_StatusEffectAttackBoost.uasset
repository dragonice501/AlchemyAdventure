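; Attack boost status effect that raises the owning character's Might while active.
; Activate adds a truncated EffectModifier fraction of base Might to the Augmented value, leaving Base untouched.
; End subtracts the same formula, recomputed from the current base and modifier rather than a stored amount.
; EffectFloat also scales the parent's returned float by EffectModifier.
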(event EventBeginPlay)

(fn ConstructionScript)

(fn Activate
  (bind _owningcharacter (Variables|Default|GetOwningCharacter))
  (bind _ac_characterattributes (Variables|/Game/Blueprints/Characters/BP_CharacterBase.BP_CharacterBase_C|GetAC_CharacterAttributes _owningcharacter))
  (|CallParentFunction)
  (Variables|/Game/Blueprints/Components/AC_AttributesBase.AC_AttributesBase_C|SetMightC _ac_characterattributes (Utilities|Struct|MakeS_AttributeCore (.base (Variables|/Game/Blueprints/Components/AC_AttributesBase.AC_AttributesBase_C|GetMightC _ac_characterattributes)) (+ (.augmented (Variables|/Game/Blueprints/Components/AC_AttributesBase.AC_AttributesBase_C|GetMightC _ac_characterattributes)) (Math|Float|Truncate (* (.base (Variables|/Game/Blueprints/Components/AC_AttributesBase.AC_AttributesBase_C|GetMightC _ac_characterattributes)) (Variables|Default|GetEffectModifier)))))))

(fn EffectFloat
  (params (InFloat :type Float%20%28double-precision%29))
  (bind _outfloat (|CallParentFunction InFloat))
  (return (* _outfloat (Variables|Default|GetEffectModifier))))

(fn End
  (bind _owningcharacter (Variables|Default|GetOwningCharacter))
  (bind _ac_characterattributes (Variables|/Game/Blueprints/Characters/BP_CharacterBase.BP_CharacterBase_C|GetAC_CharacterAttributes _owningcharacter))
  (|CallParentFunction)
  (Variables|/Game/Blueprints/Components/AC_AttributesBase.AC_AttributesBase_C|SetMightC _ac_characterattributes (Utilities|Struct|MakeS_AttributeCore (.base (Variables|/Game/Blueprints/Components/AC_AttributesBase.AC_AttributesBase_C|GetMightC _ac_characterattributes)) (- (.augmented (Variables|/Game/Blueprints/Components/AC_AttributesBase.AC_AttributesBase_C|GetMightC _ac_characterattributes)) (Math|Float|Truncate (* (.base (Variables|/Game/Blueprints/Components/AC_AttributesBase.AC_AttributesBase_C|GetMightC _ac_characterattributes)) (Variables|Default|GetEffectModifier)))))))