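; Base Blueprint for status effects on characters, providing shared state and overridable hooks.
; Activate casts its owner to BP_CharacterBase and caches it as the owning character.
; Setters store duration, modifier and effect time, resetting the remaining time, which DecreaseTimeRemaining subtracts from when called, with no expiry check.
; EffectFloat (returns zero) and End (empty) are stubs, and the event graph has no active logic.
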(event EventBeginPlay)

(event Collision|EventActorBeginOverlap
  (params (OtherActor :type Actor%20Object%20Reference)))

(fn ConstructionScript)

(fn Activate
  (bind _asbp_character_base (Utilities|Casting|CastToBP_CharacterBase (Components|GetOwner)))
  (Variables|Default|SetOwningCharacter _asbp_character_base))

(fn SetEffectTime
  (params (Time :type Float%20%28double-precision%29))
  (bind _output_get (Variables|Default|SetEffectTime Time))
  (Variables|Default|SetEffectTimeRemaining _output_get))

(fn DecreaseTimeRemaining
  (params (Time :type Float%20%28double-precision%29))
  (Variables|Default|SetEffectTimeRemaining (- (Variables|Default|GetEffectTimeRemaining) Time)))

(fn EffectFloat
  (params (InFloat :type Float%20%28double-precision%29))
  (return 0.0))

(fn SetEffectVariables
  (params (Duration :type E_EffectDuration%20Enum :default "NewEnumerator0") (Modifier :type Float%20%28double-precision%29) (Time :type Float%20%28double-precision%29))
  (Variables|Default|SetEffectDuration Duration)
  (Variables|Default|SetEffectModifier Modifier)
  (bind _output_get (Variables|Default|SetEffectTime Time))
  (Variables|Default|SetEffectTimeRemaining _output_get))

(fn End)