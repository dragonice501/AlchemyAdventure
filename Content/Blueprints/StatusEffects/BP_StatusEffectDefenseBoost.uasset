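; Status effect Blueprint that temporarily boosts the owning character's physical resistance.
; Activate adds the base resistance scaled by EffectModifier, truncated to an integer, to the Augmented value, leaving Base untouched.
; End recomputes the same amount from the current base and modifier and subtracts it, after calling the parent logic as Activate does.
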(event EventBeginPlay
  (|CallParentFunction) ; This node is disabled and will not be called.\nDrag off pins to build functionality.
)

(event Collision|EventActorBeginOverlap
  (params (OtherActor :type Actor%20Object%20Reference))
  (|CallParentFunction OtherActor) ; This node is disabled and will not be called.\nDrag off pins to build functionality.
)

(event EventTick
  (params (DeltaSeconds :type Float%20%28single-precision%29)))

(fn ConstructionScript
  (|CallParentFunction))

(fn Activate
  (bind _owningcharacter (Variables|Default|GetOwningCharacter))
  (bind _ac_characterattributes (Variables|/Game/Blueprints/Characters/BP_CharacterBase.BP_CharacterBase_C|GetAC_CharacterAttributes _owningcharacter))
  (|CallParentFunction)
  (Variables|/Game/Blueprints/Components/AC_AttributesBase.AC_AttributesBase_C|SetPhysicalResistance _ac_characterattributes (Utilities|Struct|MakeS_AttributeCore (.base (Variables|/Game/Blueprints/Components/AC_AttributesBase.AC_AttributesBase_C|GetPhysicalResistance _ac_characterattributes)) (+ (.augmented (Variables|/Game/Blueprints/Components/AC_AttributesBase.AC_AttributesBase_C|GetPhysicalResistance _ac_characterattributes)) (Math|Float|Truncate (* (.base (Variables|/Game/Blueprints/Components/AC_AttributesBase.AC_AttributesBase_C|GetPhysicalResistance _ac_characterattributes)) (Variables|Default|GetEffectModifier)))))))

(fn End
  (bind _owningcharacter (Variables|Default|GetOwningCharacter))
  (bind _ac_characterattributes (Variables|/Game/Blueprints/Characters/BP_CharacterBase.BP_CharacterBase_C|GetAC_CharacterAttributes _owningcharacter))
  (|CallParentFunction)
  (Variables|/Game/Blueprints/Components/AC_AttributesBase.AC_AttributesBase_C|SetPhysicalResistance _ac_characterattributes (Utilities|Struct|MakeS_AttributeCore (.base (Variables|/Game/Blueprints/Components/AC_AttributesBase.AC_AttributesBase_C|GetPhysicalResistance _ac_characterattributes)) (- (.augmented (Variables|/Game/Blueprints/Components/AC_AttributesBase.AC_AttributesBase_C|GetPhysicalResistance _ac_characterattributes)) (Math|Float|Truncate (* (.base (Variables|/Game/Blueprints/Components/AC_AttributesBase.AC_AttributesBase_C|GetPhysicalResistance _ac_characterattributes)) (Variables|Default|GetEffectModifier)))))))