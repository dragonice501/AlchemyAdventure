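; Base melee weapon Blueprint that damages characters its capsule overlaps while a swing is active.
; EnableCollision clears the hit list and turns on query collision, and DisableCollision turns it off, as it is at BeginPlay.
; Overlapped BPI_Character actors other than the owner are hit once per activation, receiving damage from CalculateDamage using attacker, target and base damage.
; Each hit also drains the owner's stamina.
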(event OnComponentBeginOverlap(Capsule)
  (params (OverlappedComponent :type Primitive%20Component%20Object%20Reference) (OtherActor :type Actor%20Object%20Reference) (OtherComp :type Primitive%20Component%20Object%20Reference) (OtherBodyIndex :type Integer) (bFromSweep :type Boolean) (SweepResult :type Hit%20Result%20Structure%20%28by%20ref%29))
  (bind _hitenemies (Variables|Default|GetHitEnemies))
  (if (Utilities|DoesObjectImplementInterface OtherActor "/Game/Blueprints/Interfaces/BPI_Character.BPI_Character_C")
    (if (and (!= OtherActor (Variables|Default|GetOwningCharacter)) (not (Utilities|Array|ContainsItem _hitenemies OtherActor)))
      (Utilities|Array|Add _hitenemies OtherActor)
      (bind _outdamage (CallFunction|CalculateDamage (Variables|Default|GetOwningCharacter) OtherActor (Variables|Default|GetBaseDamage)))
      (Game|Damage|ApplyDamage OtherActor _outdamage 0 0)
      (Class|BPIPlayerCharacter|DrainStamina(Message) (Variables|Default|GetOwningCharacter) (Variables|Default|GetStaminaDrain)))))

(event EventBeginPlay
  (Collision|SetCollisionEnabled (Variables|Default|GetCapsule) "NoCollision"))

(event EventEnableCollision
  (Utilities|Array|Clear (Variables|Default|GetHitEnemies))
  (Collision|SetCollisionEnabled (Variables|Default|GetCapsule) "QueryOnly"))

(event EventDisableCollision
  (Collision|SetCollisionEnabled (Variables|Default|GetCapsule) "NoCollision"))

(event EventSetOwningCharacter
  (params (Owner :type Actor%20Object%20Reference))
  (Variables|Default|SetOwningCharacter Owner))

(fn ConstructionScript)