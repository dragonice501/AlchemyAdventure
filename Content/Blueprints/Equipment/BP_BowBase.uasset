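; Base bow weapon Blueprint that fires arrows for the character holding it.
; FireArrow spawns a BP_WoodArrow at the ArrowSpawn component's location, facing along the owning character's actor rotation, with that character as instigator.
; GetWeaponType reports a fixed weapon-type enum value, and no Tick or BeginPlay logic is active.
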(event EventBeginPlay
  (|CallParentFunction) ; This node is disabled and will not be called.\nDrag off pins to build functionality.
)

(event Collision|EventActorBeginOverlap
  (params (OtherActor :type Actor%20Object%20Reference))
  (|CallParentFunction OtherActor) ; This node is disabled and will not be called.\nDrag off pins to build functionality.
)

(event EventTick
  (params (DeltaSeconds :type Float%20%28single-precision%29))
  (|CallParentFunction DeltaSeconds) ; This node is disabled and will not be called.\nDrag off pins to build functionality.
)

(event EventFireArrow
  (bind _owningcharacter (Variables|Default|GetOwningCharacter))
  (Game|SpawnActorfromClass "/Game/Blueprints/Equipment/BP_WoodArrow.BP_WoodArrow_C" (Math|Transform|MakeTransform (Transformation|GetWorldLocation (Variables|Default|GetArrowSpawn)) (Transformation|GetActorRotation _owningcharacter) "1.000000,1.000000,1.000000") "Undefined" "MultiplyWithRoot" 0 _owningcharacter))

(fn ConstructionScript
  (|CallParentFunction))

(fn GetWeaponType
  (return "NewEnumerator3"))