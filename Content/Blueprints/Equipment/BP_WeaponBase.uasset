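; BP_WeaponBase is a weapon base that damages characters overlapped by its capsule.
; EnableCollision clears the HitEnemies list and turns on query-only collision, and DisableCollision turns it off, as does BeginPlay.
; Each overlap skips the owner and already-hit actors, so a target is hit once per activation.
; New hits pass base damage through CalculateDamage into ApplyDamage, then drain the owner's stamina per target hit.
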(event OnComponentBeginOverlap(Capsule)
  (params (OverlappedComponent :type Primitive%20Component%20Object%20Reference) (OtherActor :type Actor%20Object%20Reference) (OtherComp :type Primitive%20Component%20Object%20Reference) (OtherBodyIndex :type Integer) (bFromSweep :type Boolean) (SweepResult :type Hit%20Result%20Structure%20%28by%20ref%29))
  (bind _hitenemies (Variables|Default|GetHitEnemies))
  (bind _asbp_character_base (Utilities|Casting|CastToBP_CharacterBase OtherActor))
  (if (and (!= _asbp_character_base (Variables|Default|GetOwningCharacter)) (not (Utilities|Array|ContainsItem _hitenemies OtherActor)))
    (Utilities|Array|Add _hitenemies OtherActor)
    (bind _outdamage (CallFunction|CalculateDamage (Variables|Default|GetOwningCharacter) _asbp_character_base (Variables|Default|GetBaseDamage)))
    (Game|Damage|ApplyDamage OtherActor _outdamage 0 0)
    (Default|DrainStamina (Variables|Default|GetOwningCharacter) (Variables|Default|GetStaminaDrain))))

(event EventBeginPlay
  (Collision|SetCollisionEnabled (Variables|Default|GetCapsule) "NoCollision"))

(fn ConstructionScript)

(fn EnableCollision
  (Utilities|Array|Clear (Variables|Default|GetHitEnemies))
  (Collision|SetCollisionEnabled (Variables|Default|GetCapsule) "QueryOnly"))

(fn DisableCollision
  (Collision|SetCollisionEnabled (Variables|Default|GetCapsule) "NoCollision"))