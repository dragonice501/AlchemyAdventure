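; Base arrow projectile that damages enemies on contact and expires a few seconds after spawning.
; A setter stores the parent bow and owning character.
; When its sphere overlaps an actor implementing BPI_Enemy, it adds the bow's physical attack stat to its own damage, applies that as the owner's damage, then destroys itself.
; Overlaps with any other actor are ignored.
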(event OnComponentBeginOverlap(Sphere)
  (params (OverlappedComponent :type Primitive%20Component%20Object%20Reference) (OtherActor :type Actor%20Object%20Reference) (OtherComp :type Primitive%20Component%20Object%20Reference) (OtherBodyIndex :type Integer) (bFromSweep :type Boolean) (SweepResult :type Hit%20Result%20Structure%20%28by%20ref%29))
  (bind _owningcharacter (Variables|Default|GetOwningCharacter))
  (if (Utilities|DoesObjectImplementInterface OtherActor "/Game/Blueprints/Interfaces/BPI_Enemy.BPI_Enemy_C")
    (bind _stats (Class|BPIWeapon|GetWeaponStats(Message) (Variables|Default|GetParentBow)))
    (Game|Damage|ApplyDamage OtherActor (+ (.attackphysical _stats) (Variables|Default|GetDamage)) (Pawn|GetController _owningcharacter) _owningcharacter)
    (Actor|DestroyActor)))

(event EventBeginPlay
  (|CallParentFunction)
  (Actor|SetLifeSpan 5.0))

(event EventSetParentBow
  (params (ParentBow :type Actor%20Object%20Reference) (OwningCharacter :type Pawn%20Object%20Reference))
  (Variables|Default|SetParentBow ParentBow)
  (Variables|Default|SetOwningCharacter OwningCharacter))

(fn ConstructionScript
  (|CallParentFunction))