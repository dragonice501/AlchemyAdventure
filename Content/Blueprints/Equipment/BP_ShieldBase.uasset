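; Base shield equipment Blueprint that provides a mostly stubbed set of weapon functions.
; It disables collision on its static mesh at BeginPlay and stores the owning character when assigned.
; Secondary action start and end only check that the owner is valid, with no behavior attached.
; Montage and stats getters return empty, stamina drain returns zero, and the weapon type is the enum's NewEnumerator0 entry.
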(event EventBeginPlay
  (Collision|SetCollisionEnabled (Variables|Default|GetStaticMesh) "NoCollision"))

(event EventWeaponStartSecondaryAction
  (Variables|Default|GetOwningCharacter
    (:then)
    (:else)))

(event EventWeaponEndSecondaryAction
  (Variables|Default|GetOwningCharacter
    (:then)
    (:else)))

(event EventSetOwningCharacter
  (params (Owner :type Character%20Object%20Reference))
  (Variables|Default|SetOwningCharacter Owner))

(fn ConstructionScript)

(fn GetAttackMontage
  (return 0))

(fn GetBlockMontage
  (return 0))

(fn GetStaminaDrain
  (return 0.0))

(fn GetWeaponStats
  (return ""))

(fn GetWeaponType
  (return "NewEnumerator0"))