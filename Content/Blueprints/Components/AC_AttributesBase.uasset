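; AC_AttributesBase is a base attributes component that holds character stats and exposes them through grouped getter functions.
; Core and secondary getters return stored variables: seven primary stats from Vigor to Agility, plus health and stamina, with the Stamina output fed by StaminaMax.
; The defense getter returns zero for physical, strike, slash and pierce resistance.
; It contains no calculation or active event logic.
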(event EventBeginPlay)

(event EventTick
  (params (DeltaSeconds :type Float%20%28single-precision%29)))

(fn GetCoreAttributes
  (return (Variables|AttributesCore|GetVigor) (Variables|AttributesCore|GetEndurance) (Variables|AttributesCore|GetMight) (Variables|AttributesCore|GetResolve) (Variables|AttributesCore|GetCognition) (Variables|AttributesCore|GetPeity) (Variables|AttributesCore|GetAgility)))

(fn GetSecondaryAttributes
  (return (Variables|AttributesSecondary|GetHealth) (Variables|AttributesSecondary|GetMaxHealth) (Variables|AttributesSecondary|GetStaminaMax)))

(fn GetDefenseAttributes
  (return 0.0 0.0 0.0 0.0))