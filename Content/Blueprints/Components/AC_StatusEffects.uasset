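; Character component that manages status effects as spawned actors, sorted into attack, defense and health types.
; Attack and defense effects are stored, attached to the owner and shown via the character's widget call, but only attack and instant health effects get activated.
; Tick counts down timed effects and destroys expired ones.
; Damage passes through each attack effect in turn, while the might multiplier adds up their bonuses.
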(event EventBeginPlay
  (bind _asbp_character_base (Utilities|Casting|CastToBP_CharacterBase (Components|GetOwner)))
  (Variables|Default|SetCharacter _asbp_character_base))

(event EventTick
  (params (DeltaSeconds :type Float%20%28single-precision%29))
  (CallFunction|UpdateAttackEffects DeltaSeconds)
  (CallFunction|UpdateDefenseEffects DeltaSeconds))

(fn AddStatusEffect
  (params (StatusEffect :type BP%20Status%20Effect%20Base%20Class%20Reference) (Owner :type Actor%20Object%20Reference) (EffectTime :type Float%20%28double-precision%29))
  (bind _returnvalue (Game|SpawnActorfromClass StatusEffect (Transformation|GetActorTransform Owner) "Undefined" "MultiplyWithRoot" Owner 0))
  (switch Utilities|FlowControl|Switch|SwitchonE_EffectType (Variables|/Game/Blueprints/StatusEffects/BP_StatusEffectBase.BP_StatusEffectBase_C|GetEffectType _returnvalue)
    (:NewEnumerator1
      (Default|SetEffectTime _returnvalue EffectTime)
      (Utilities|Array|Add (Variables|Default|GetAttackEffects) _returnvalue)
      (Default|Activate _returnvalue)
      (Transformation|AttachActorToActor _returnvalue Owner "None" "KeepRelative" "KeepRelative" "KeepRelative" true :!label _label)
      (Default|AddStatusEffect (Variables|Default|GetCharacter) (Variables|/Game/Blueprints/StatusEffects/BP_StatusEffectBase.BP_StatusEffectBase_C|GetEffectWidget _returnvalue) (Variables|/Game/Blueprints/StatusEffects/BP_StatusEffectBase.BP_StatusEffectBase_C|GetEffectTime _returnvalue)))
    (:NewEnumerator2
      (Default|SetEffectTime _returnvalue EffectTime)
      (Utilities|Array|Add (Variables|Default|GetDefenseEffects) _returnvalue)
      (goto _label))
    (:NewEnumerator4
      (switch Utilities|FlowControl|Switch|SwitchonE_EffectDuration (Variables|/Game/Blueprints/StatusEffects/BP_StatusEffectBase.BP_StatusEffectBase_C|GetEffectDuration _returnvalue)
        (:NewEnumerator2
          (Default|Activate _returnvalue))))))

(fn EffectDamage
  (params (InDamage :type Float%20%28double-precision%29))
  (LocalVariables|SetDamage InDamage)
  (for _array_element (Variables|Default|GetAttackEffects)
    (bind _outfloat (Default|EffectFloat _array_element (LocalVariables|GetDamage)))
    (LocalVariables|SetDamage _outfloat))
  (return (LocalVariables|GetDamage)))

(fn GetMightMultiplier
  (LocalVariables|SetMightMultiplier 1.0)
  (for _array_element (Variables|Default|GetAttackEffects)
    (LocalVariables|SetMightMultiplier (+ (LocalVariables|GetMightMultiplier) (- (Variables|/Game/Blueprints/StatusEffects/BP_StatusEffectBase.BP_StatusEffectBase_C|GetEffectMultiplier _array_element) 1.0))))
  (return (LocalVariables|GetMightMultiplier)))

(fn UpdateAttackEffects
  (params (Time :type Float%20%28double-precision%29))
  (bind _attackeffects (Variables|Default|GetAttackEffects))
  (for _array_element _attackeffects
    (if (Utilities|Enum|Equal(Enum) (Variables|/Game/Blueprints/StatusEffects/BP_StatusEffectBase.BP_StatusEffectBase_C|GetEffectDuration _array_element) "NewEnumerator1")
      (Default|DecreaseTimeRemaining _array_element Time)))
  (for _array_element_2 _attackeffects
    (if (Utilities|Enum|Equal(Enum) (Variables|/Game/Blueprints/StatusEffects/BP_StatusEffectBase.BP_StatusEffectBase_C|GetEffectDuration _array_element_2) "NewEnumerator1")
      (if (<= (Variables|/Game/Blueprints/StatusEffects/BP_StatusEffectBase.BP_StatusEffectBase_C|GetEffectTimeRemaining _array_element_2) 0.0)
        (Variables|Default|SetEffectRef _array_element_2)
        (Utilities|Array|RemoveItem _attackeffects _array_element_2)
        (Actor|DestroyActor (Variables|Default|GetEffectRef))
        (Variables|Default|SetEffectRef 0)))))

(fn UpdateDefenseEffects
  (params (Time :type Float%20%28double-precision%29))
  (bind _defenseeffects (Variables|Default|GetDefenseEffects))
  (for _array_element _defenseeffects
    (if (Utilities|Enum|Equal(Enum) (Variables|/Game/Blueprints/StatusEffects/BP_StatusEffectBase.BP_StatusEffectBase_C|GetEffectDuration _array_element) "NewEnumerator1")
      (Default|DecreaseTimeRemaining _array_element Time)))
  (for _array_element_2 _defenseeffects
    (if (Utilities|Enum|Equal(Enum) (Variables|/Game/Blueprints/StatusEffects/BP_StatusEffectBase.BP_StatusEffectBase_C|GetEffectDuration _array_element_2) "NewEnumerator1")
      (if (<= (Variables|/Game/Blueprints/StatusEffects/BP_StatusEffectBase.BP_StatusEffectBase_C|GetEffectTimeRemaining _array_element_2) 0.0)
        (Variables|Default|SetEffectRef _array_element_2)
        (Utilities|Array|RemoveItem _defenseeffects _array_element_2)
        (Actor|DestroyActor (Variables|Default|GetEffectRef))
        (Variables|Default|SetEffectRef 0)))))