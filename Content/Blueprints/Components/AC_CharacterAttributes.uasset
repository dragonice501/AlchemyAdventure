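; Actor component that holds a character's health and stamina and provides functions to change them.
; On BeginPlay it caches its owner as BP_CharacterBase.
; Health changes and stamina drains are clamped to their valid ranges, and health is also exposed as a percentage.
; Stamina recharge scales with delta time without clamping and clears the owner's RechargeStamina flag once the maximum is reached.
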(event EventBeginPlay
  (bind _asbp_character_base (Utilities|Casting|CastToBP_CharacterBase (Components|GetOwner)))
  (Variables|Default|SetCharacter _asbp_character_base))

(fn DrainStamina
  (params (StaminaDrain :type Float%20%28double-precision%29))
  (Variables|Default|SetStamina (Math|Float|Clamp(Float) (- (Variables|Default|GetStamina) StaminaDrain) 0.0 (Variables|Default|GetStaminaMax))))

(fn RechargeStamina
  (bind _output_get (Variables|Default|SetStamina (+ (Variables|Default|GetStamina) (* (Variables|Default|GetStaminaRechargeRate) (Utilities|Time|GetWorldDeltaSeconds)))))
  (if (>= _output_get (Variables|Default|GetStaminaMax))
    (Variables|/Game/Blueprints/Characters/BP_CharacterBase.BP_CharacterBase_C|SetRechargeStamina (Variables|Default|GetCharacter) false)))

(fn AddHealth
  (params (Amount :type Integer))
  (Variables|Default|SetHealth (Math|Float|Clamp(Float) (+ (Variables|Default|GetHealth) Amount) 0.0 (Variables|Default|GetMaxHealth))))

(fn GetHealthPercent
  (return (Math|Float|SafeDivide (Variables|Default|GetHealth) (Variables|Default|GetMaxHealth))))