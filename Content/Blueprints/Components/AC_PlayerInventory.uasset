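; Player inventory component that stores weapons, shields, talismans, recipes, resources and craftable usables.
; Add functions look up data table rows by name, filing weapons into sword or bow arrays and stacking resources and usables in struct-to-count maps.
; Getters address items by slot index, using map key order for stacks, and resolve crafting pairs and recipe ingredients.
; Decrements leave empty stacks until separate update events remove them with a shared index offset.
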(event EventUpdateUsables
  (bind _usables (Variables|Default|GetUsables))
  (bind _values (Utilities|Map|Values _usables))
  (for (_array_element _array_index) _values
    (if (<= _array_element 0)
      (bind _keys (Utilities|Map|Keys _usables))
      (bind _returnvalue (Utilities|Map|Remove _usables (Utilities|Array|Get(acopy) _keys (- _array_index (Variables|Default|GetIndexOffset)))))
      (if _returnvalue
        (bind _result (Math|Integer|IncrementInt (Variables|Default|GetIndexOffset)))))))

(event EventDecreaseUsableatIndex
  (params (Index :type Integer))
  (bind _usables (Variables|Default|GetUsables))
  (bind _keys (Utilities|Map|Keys _usables))
  (bind _result (Math|Integer|DecrementInt (.Value (Utilities|Map|Find _usables (Utilities|Array|Get(acopy) _keys Index))))
    (:%20%20
      (Utilities|Map|Add _usables (Utilities|Array|Get(acopy) _keys Index) _result))))

(event EventUpdateAllResources
  (bind _resources (Variables|Default|GetResources))
  (bind _values (Utilities|Map|Values _resources))
  (for (_array_element _array_index) _values
    (if (<= _array_element 0)
      (bind _keys (Utilities|Map|Keys _resources))
      (bind _returnvalue (Utilities|Map|Remove _resources (Utilities|Array|Get(acopy) _keys (- _array_index (Variables|Default|GetIndexOffset)))))
      (if _returnvalue
        (bind _result (Math|Integer|IncrementInt (Variables|Default|GetIndexOffset))))))
  (Variables|Default|SetIndexOffset 0))

(event EventDecreaseResource
  (params (Index :type Integer))
  (bind _resources (Variables|Default|GetResources))
  (bind _keys (Utilities|Map|Keys _resources))
  (bind _result (Math|Integer|DecrementInt (.Value (Utilities|Map|Find _resources (Utilities|Array|Get(acopy) _keys Index))))
    (:%20%20
      (Utilities|Map|Add _resources (Utilities|Array|Get(acopy) _keys Index) _result))))

(fn AddRecipe
  (params (Recipe :type String))
  (LocalVariables|SetFound false)
  (bind _array_element (Utilities|Array|ForEachLoopwithBreak (Variables|Default|GetRecipes) :!label _label)
    (:LoopBody
      (if (Utilities|Enum|Equal(Enum) (.name _array_element) Recipe)
        (LocalVariables|SetFound true)
        (goto _label Break)))
    (:Completed
      (if (not (LocalVariables|GetFound))
        (bind _returnvalue (Utilities|GetDataTableRow (Variables|Default|GetRecipesTable) (Utilities|String|StringToName Recipe))
          (:then
            (bind _returnvalue_2 (Utilities|Array|Add (Variables|Default|GetRecipes) _returnvalue))
            (return _returnvalue_2)))
        (else
          (return 0))))))

(fn AddResource
  (params (ResourceName :type Name :default "None"))
  (bind _resources (Variables|Default|GetResources))
  (bind _returnvalue (Utilities|GetDataTableRow (Variables|Default|GetResourcesTable) ResourceName)
    (:then
      (LocalVariables|SetResource _returnvalue)
      (bind _keys (Utilities|Map|Keys (Variables|Default|GetResources)))
      (if (!= (Utilities|Array|FindItem _keys (LocalVariables|GetResource)) -1)
        (bind _result (Math|Integer|IncrementInt (.Value (Utilities|Map|Find _resources (LocalVariables|GetResource))))
          (:%20%20
            (Utilities|Map|Add _resources (LocalVariables|GetResource) _result)
            (return (Utilities|Array|FindItem _keys (LocalVariables|GetResource)) _result)))
        (else
          (Utilities|Map|Add (Variables|Default|GetResources) (LocalVariables|GetResource) 1)
          (bind _keys_2 (Utilities|Map|Keys (Variables|Default|GetResources)))
          (return (Utilities|Array|FindItem _keys_2 (LocalVariables|GetResource)) 1))))))

(fn AddShield
  (params (ShieldName :type Name :default "None"))
  (bind _returnvalue (Utilities|GetDataTableRow (Variables|Default|GetShieldsTable) ShieldName)
    (:then
      (bind _returnvalue_2 (Utilities|Array|Add (Variables|Default|GetShields) _returnvalue))
      (return _returnvalue_2))))

(fn AddTalisman
  (params (TalismanName :type Name :default "None"))
  (bind _returnvalue (Utilities|GetDataTableRow (Variables|Default|GetTalismansTable) TalismanName)
    (:then
      (bind _returnvalue_2 (Utilities|Array|Add (Variables|Default|GetTalismans) _returnvalue))
      (return _returnvalue_2))))

(fn AddUsable
  (params (Craftable :type String))
  (bind _usables (Variables|Default|GetUsables))
  (bind _returnvalue (Utilities|GetDataTableRow (Variables|Default|GetCraftablesTable) (Utilities|String|StringToName Craftable))
    (:then
      (LocalVariables|SetNewUsable _returnvalue)
      (bind _keys (Utilities|Map|Keys (Variables|Default|GetUsables)))
      (if (!= (Utilities|Array|FindItem _keys (LocalVariables|GetNewUsable)) -1)
        (bind _result (Math|Integer|IncrementInt (.Value (Utilities|Map|Find _usables (LocalVariables|GetNewUsable))))
          (:%20%20
            (Utilities|Map|Add _usables (LocalVariables|GetNewUsable) _result)
            (return (LocalVariables|GetNewUsable) (Utilities|Array|FindItem _keys (LocalVariables|GetNewUsable)) _result)))
        (else
          (Utilities|Map|Add (Variables|Default|GetUsables) (LocalVariables|GetNewUsable) 1)
          (bind _keys_2 (Utilities|Map|Keys (Variables|Default|GetUsables)))
          (return (LocalVariables|GetNewUsable) (Utilities|Array|FindItem _keys_2 (LocalVariables|GetNewUsable)) 1))))))

(fn AddWeapon
  (params (WeaponName :type Name :default "None"))
  (bind _returnvalue (Utilities|GetDataTableRow (Variables|Default|GetWeaponsTable) WeaponName)
    (:then
      (switch Utilities|FlowControl|Switch|SwitchonE_WeaponType (.EquipmentType (Utilities|Struct|BreakS_Weapon _returnvalue))
        (:NewEnumerator0
          (bind _returnvalue_2 (Utilities|Array|Add (Variables|Default|GetSwords) _returnvalue))
          (return _returnvalue_2 (.EquipmentType (Utilities|Struct|BreakS_Weapon _returnvalue))))
        (:NewEnumerator3
          (bind _returnvalue_3 (Utilities|Array|Add (Variables|Default|GetBows) _returnvalue))
          (return _returnvalue_3 (.EquipmentType (Utilities|Struct|BreakS_Weapon _returnvalue))))))))

(fn GetBows
  (return (Variables|Default|GetBows)))

(fn GetCraftablefromResources
  (params (IndexOne :type Integer) (IndexTwo :type Integer))
  (bind _keys (Utilities|Map|Keys (Variables|Default|GetResources)))
  (bind _output_get (LocalVariables|SetResourcesArray _keys))
  (if (Utilities|Enum|Equal(Enum) (.combinableone (Utilities|Array|Get(acopy) _output_get IndexOne)) (.name (Utilities|Array|Get(acopy) (LocalVariables|GetResourcesArray) IndexTwo)))
    (bind _returnvalue (Utilities|GetDataTableRow (Variables|Default|GetCraftablesTable) (Utilities|String|StringToName (.combineresultone (Utilities|Array|Get(acopy) _output_get IndexOne))))
      (:then
        (return _returnvalue)))
    (elif (Utilities|Enum|Equal(Enum) (.combinabletwo (Utilities|Array|Get(acopy) _output_get IndexOne)) (.name (Utilities|Array|Get(acopy) (LocalVariables|GetResourcesArray) IndexTwo)))
      (bind _returnvalue_2 (Utilities|GetDataTableRow (Variables|Default|GetCraftablesTable) (Utilities|String|StringToName (.combineresulttwo (Utilities|Array|Get(acopy) _output_get IndexOne))))
        (:then
          (return _returnvalue_2)))
      (else
        (return "")))))

(fn GetRecipefromInvIndex
  (params (Index :type Integer))
  (bind _recipes (Variables|Default|GetRecipes))
  (if (< Index (Utilities|Array|Length _recipes))
    (return (Utilities|Array|Get(acopy) _recipes Index))
    (else
      (return ""))))

(fn GetRecipeIngredient
  (params (Ingredient :type String))
  (bind _resources (Variables|Default|GetResources))
  (if (Utilities|Enum|NotEqual(Enum) Ingredient "")
    (bind _returnvalue (Utilities|GetDataTableRow (Variables|Default|GetResourcesTable) (Utilities|String|StringToName Ingredient))
      (:then
        (if (.ReturnValue (Utilities|Map|Find _resources _returnvalue))
          (bind _keys (Utilities|Map|Keys _resources))
          (return (Utilities|Array|FindItem _keys _returnvalue) (.Value (Utilities|Map|Find _resources _returnvalue)) (.ResourceImage (Utilities|Struct|BreakS_Resource _returnvalue)))
          (else
            (return -1 0 (.ResourceImage (Utilities|Struct|BreakS_Resource _returnvalue)))))))
    (else
      (return 0 0 0))))

(fn GetResourceandCount
  (params (Index :type Integer))
  (bind _resources (Variables|Default|GetResources))
  (bind _keys (Utilities|Map|Keys _resources))
  (if (< Index (Utilities|Array|Length _keys))
    (bind _values (Utilities|Map|Values _resources))
    (return (Utilities|Array|Get(acopy) _values Index) (.resourceimage (Utilities|Array|Get(acopy) _keys Index)))
    (else
      (return 0 0))))

(fn GetResourcefromInvIndex
  (params (Index :type Integer))
  (bind _keys (Utilities|Map|Keys (Variables|Default|GetResources)))
  (if (< Index (Utilities|Array|Length _keys))
    (return (Utilities|Array|Get(acopy) _keys Index))))

(fn GetResources
  (return (Variables|Default|GetResources)))

(fn GetShieldfromInvIndex
  (params (Index :type Integer))
  (bind _shields (Variables|Default|GetShields))
  (if (< Index (Utilities|Array|Length _shields))
    (return (Utilities|Array|Get(acopy) _shields Index))
    (else
      (return ""))))

(fn GetShields
  (return (Variables|Default|GetShields)))

(fn GetSwords
  (return (Variables|Default|GetSwords)))

(fn GetTalismanfromInvIndex
  (params (Index :type Integer))
  (bind _talismans (Variables|Default|GetTalismans))
  (if (< Index (Utilities|Array|Length _talismans))
    (return (Utilities|Array|Get(acopy) _talismans Index))
    (else
      (return ""))))

(fn GetTalismans
  (return (Variables|Default|GetTalismans)))

(fn GetUsableandCountfromInvIndex
  (params (Index :type Integer))
  (bind _usables (Variables|Default|GetUsables))
  (if (!= Index -1)
    (bind _keys (Utilities|Map|Keys _usables))
    (if (< Index (Utilities|Array|Length _keys))
      (bind _values (Utilities|Map|Values _usables))
      (return (.image (Utilities|Array|Get(acopy) _keys Index)) (Utilities|Array|Get(acopy) _values Index))
      (else
        (return 0 0)))))

(fn GetUsablefromInvIndex
  (params (Index :type Integer))
  (bind _keys (Utilities|Map|Keys (Variables|Default|GetUsables)))
  (if (< Index (Utilities|Array|Length _keys))
    (return (Utilities|Array|Get(acopy) _keys Index))
    (else
      (return ""))))

(fn GetUsables
  (return (Variables|Default|GetUsables)))

(fn GetWeapon
  (params (Index :type Integer) (WeaponType :type E_WeaponType%20Enum :default "NewEnumerator0"))
  (bind _swords (Variables|Default|GetSwords))
  (bind _bows (Variables|Default|GetBows))
  (switch Utilities|FlowControl|Switch|SwitchonE_WeaponType WeaponType
    (:NewEnumerator0
      (if (< Index (Utilities|Array|Length _swords))
        (return (Utilities|Array|Get(acopy) _swords Index))
        (else
          (return ""))))
    (:NewEnumerator3
      (if (< Index (Utilities|Array|Length _bows))
        (return (Utilities|Array|Get(acopy) _bows Index))
        (else
          (return ""))))))

(fn GetWeaponfromInvIndex
  (params (Index :type Integer) (WeaponType :type E_WeaponType%20Enum :default "NewEnumerator0"))
  (bind _swords (Variables|Default|GetSwords))
  (bind _bows (Variables|Default|GetBows))
  (switch Utilities|FlowControl|Switch|SwitchonE_WeaponType WeaponType
    (:NewEnumerator0
      (if (< Index (Utilities|Array|Length _swords))
        (return (Utilities|Array|Get(acopy) _swords Index))
        (else
          (return ""))))
    (:NewEnumerator3
      (if (< Index (Utilities|Array|Length _bows))
        (return (Utilities|Array|Get(acopy) _bows Index))
        (else
          (return ""))))))

(fn GetWeaponImage
  (params (Index :type Integer) (WeaponType :type E_WeaponType%20Enum :default "NewEnumerator0"))
  (bind _swords (Variables|Default|GetSwords))
  (bind _bows (Variables|Default|GetBows))
  (switch Utilities|FlowControl|Switch|SwitchonE_WeaponType WeaponType
    (:NewEnumerator0
      (if (and (< Index (Utilities|Array|Length _swords)) (!= Index -1))
        (return (.equipmentimage (Utilities|Array|Get(acopy) _swords Index)))
        (else
          (return 0))))
    (:NewEnumerator3
      (if (and (< Index (Utilities|Array|Length _bows)) (!= Index -1))
        (return (.equipmentimage (Utilities|Array|Get(acopy) _bows Index)))
        (else
          (return 0))))))

(fn HasResourceatInvIndex
  (params (Index :type Integer))
  (return (> (Utilities|Map|Length (Variables|Default|GetResources)) Index)))