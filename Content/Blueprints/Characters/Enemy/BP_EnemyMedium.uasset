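; BP_EnemyMedium is a medium enemy character that adds an overhead health bar widget and perception-based player detection to its parent class.
; On BeginPlay it binds the WBP_EnemyHealthBar widget to itself and hides it.
; Show and hide events toggle the bar's visibility, deferring to the parent's show logic when not locked.
; Successfully sensing BP_MainCharacter through AI perception sets it as the seen target.
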(event OnTargetPerceptionUpdated(AIPerception)
  (params (Actor :type Actor%20Object%20Reference) (Stimulus :type AI%20Stimulus%20Structure))
  (bind _asbp_main_character (Utilities|Casting|CastToBP_MainCharacter Actor))
  (if (.bSuccessfullySensed (Utilities|Struct|BreakAIStimulus Stimulus))
    (Class|Enemy|SetTargetCharacter _asbp_main_character true)))

(event EventBeginPlay
  (bind _healthbar (Variables|Default|GetHealthBar))
  (bind _returnvalue (UserInterface|GetUserWidgetObject _healthbar))
  (bind _aswbp_enemy_health_bar (Utilities|Casting|CastToWBP_EnemyHealthBar _returnvalue))
  (Variables|/Game/Blueprints/HUD/WBP_EnemyHealthBar.WBP_EnemyHealthBar_C|SetEnemy _aswbp_enemy_health_bar self)
  (Widget|SetVisibility _returnvalue "Hidden"))

(event EventShowHealthBar
  (params (Locked :type Boolean))
  (Widget|SetVisibility (UserInterface|GetUserWidgetObject (Variables|Default|GetHealthBar)) "Visible")
  (if (not Locked)
    (|CallParentFunction false)))

(event EventHideHealthBar
  (Widget|SetVisibility (UserInterface|GetUserWidgetObject (Variables|Default|GetHealthBar)) "Hidden"))

(fn ConstructionScript
  (|CallParentFunction))