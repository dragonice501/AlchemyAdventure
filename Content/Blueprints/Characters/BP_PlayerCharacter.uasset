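; BP_PlayerCharacter is the player's character Blueprint, extending a parent character with inventory, interaction and HUD hooks.
; BeginPlay creates and stores a player inventory component, which GetInventory exposes.
; Interactable add/remove refreshes the interact widget, and DrainStamina pushes the stamina percentage to the HUD.
; AdjustControlRotation adds 360 input to negative pitch, checking yaw only in that branch; its direct SetControlRotation nodes are disconnected.
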(event EventBeginPlay
  (|CallParentFunction)
  (CallFunction|CreateInventoryComponent))

(fn ConstructionScript
  (|CallParentFunction))

(fn AddInteractable0
  (params (Interactable :type Actor%20Object%20Reference))
  (CallFunction|SetInteractWidget))

(fn RemoveInteractable0
  (params (Interactable :type Actor%20Object%20Reference))
  (CallFunction|SetInteractWidget))

(fn AdjustControlRotation
  (bind _returnvalue (Pawn|GetControlRotation :!class /Script/Engine.Pawn))
  (if (< (.pitch _returnvalue) 0.0)
    (Pawn|Input|AddControllerPitchInput 3.6e+02)
    (if (< (.yaw _returnvalue) 0.0)
      (Pawn|Input|AddControllerYawInput 3.6e+02))))

(fn DrainStamina
  (params (StaminaDrain :type Float%20%28double-precision%29))
  (|CallParentFunction StaminaDrain)
  (Default|SetPlayerStamina (Variables|Default|GetHUD) (CallFunction|GetStaminaPercent)))

(fn CreateInventoryComponent
  (|CallParentFunction)
  (bind _returnvalue (Game|AddComponentbyClass "/Game/Blueprints/Components/AC_PlayerInventory.AC_PlayerInventory_C"))
  (Variables|Default|SetPlayerInventory _returnvalue))

(fn GetInventory
  (return (Variables|Default|GetAC_PlayerInventory)))