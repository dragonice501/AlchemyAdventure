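; Base enemy character with a health bar, player detection, lock-on point and item drop on death.
; PlayerDetection overlaps register the enemy with the other actor and set or clear the player as the AI controller's blackboard combat target.
; Damage reveals the bar, updating health and damage numbers.
; Death plays a montage and disables collision; a separate DeathEnd event releases player lock-on, freezes animation and spawns a random pickup.
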(event OnComponentBeginOverlap(PlayerDetection)
  (params (OverlappedComponent :type Primitive%20Component%20Object%20Reference) (OtherActor :type Actor%20Object%20Reference) (OtherComp :type Primitive%20Component%20Object%20Reference) (OtherBodyIndex :type Integer) (bFromSweep :type Boolean) (SweepResult :type Hit%20Result%20Structure%20%28by%20ref%29))
  (Class|BPICombat|AddEnemy(Message) OtherActor self)
  (if (Utilities|DoesObjectImplementInterface OtherActor "/Game/Blueprints/Interfaces/BPI_Player.BPI_Player_C")
    (bind _asbp_character_base (Utilities|Casting|CastToBP_CharacterBase OtherActor))
    (Variables|Default|SetPlayerCharacter _asbp_character_base)
    (Default|SetBlackBoardCombatTarget (Variables|Default|GetEnemyController) OtherActor)))

(event OnComponentEndOverlap(PlayerDetection)
  (params (OverlappedComponent :type Primitive%20Component%20Object%20Reference) (OtherActor :type Actor%20Object%20Reference) (OtherComp :type Primitive%20Component%20Object%20Reference) (OtherBodyIndex :type Integer))
  (Class|BPICombat|RemoveEnemy(Message) OtherActor self)
  (if (Utilities|DoesObjectImplementInterface OtherActor "/Game/Blueprints/Interfaces/BPI_Player.BPI_Player_C")
    (Variables|Default|SetPlayerCharacter 0)
    (Default|SetBlackBoardCombatTarget (Variables|Default|GetEnemyController))))

(event Custom|SpawnPickup
  (bind _itemdrops (Variables|Default|GetItemDrops))
  (bind _returnvalue (Game|SpawnActorfromClass "/Game/Blueprints/Pickups/BP_ItemDrop.BP_ItemDrop_C" (Transformation|GetActorTransform) "Undefined" "MultiplyWithRoot" 0 0))
  (Default|SetDropItem _returnvalue (Utilities|Array|Get(acopy) _itemdrops (Math|Random|RandomInteger (- (Utilities|Array|Length _itemdrops) 1)))))

(event EventBeginPlay
  (CallFunction|SetHealthBarVisibility false)
  (CallFunction|InitHealthBar)
  (bind _asbp_enemy_controller_base (Utilities|Casting|CastToBP_EnemyControllerBase (Pawn|GetController)))
  (Variables|Default|SetEnemyController _asbp_enemy_controller_base))

(event EventDeathEnd
  (bind _playercharacter (Variables|Default|GetPlayerCharacter))
  (CallFunction|SetHealthBarVisibility false)
  (Default|UnlockonEnemy _playercharacter self)
  (Default|EndCameraLookatEnemy _playercharacter)
  (Variables|/Script/Engine.SkeletalMeshComponent|SetbPauseAnims (Variables|Character|GetMesh) true)
  (CallFunction|SpawnPickup)
  (Collision|SetCollisionEnabled (Variables|Default|GetPlayerDetection) "NoCollision"))

(event EventDeathStart
  (Animation|Montage|PlayMontage (Variables|Character|GetMesh) (Variables|Default|GetMontageDeath)
    (:then
      (Collision|SetCollisionEnabled (Variables|Default|GetCapsuleComponent) "NoCollision")
      (Collision|SetCollisionEnabled (Variables|Character|GetMesh) "NoCollision"))))

(event EventSetHealthBarVisibility
  (params (Visibility :type Boolean))
  (Rendering|SetVisibility (Variables|Default|GetHealthBar) Visibility false))

(event Game|Damage|EventAnyDamage
  (params (Damage :type Float%20%28single-precision%29) (DamageType :type Damage%20Type%20Object%20Reference) (InstigatedBy :type Controller%20Object%20Reference) (DamageCauser :type Actor%20Object%20Reference))
  (CallFunction|SetHealthBarVisibility true)
  (CallFunction|TakeDamage Damage))

(event EventStartEnemyHealthHide
  (Utilities|FlowControl|Delay 1.0)
  (if (!= (Variables|/Game/Blueprints/Characters/BP_CharacterBase.BP_CharacterBase_C|GetTargetCharacter (Variables|Default|GetPlayerCharacter)) self)
    (CallFunction|SetHealthBarVisibility false)))

(fn ConstructionScript
  (|CallParentFunction))

(fn TakeDamage
  (params (Damage :type Float%20%28double-precision%29))
  (bind _healthbarwidget (Variables|Default|GetHealthBarWidget))
  (bind _ac_characterattributes (Variables|Default|GetAC_CharacterAttributes))
  (|CallParentFunction Damage)
  (Default|ShowDamageNumber _healthbarwidget Damage)
  (Default|SetHealthPercent _healthbarwidget (Math|Float|SafeDivide (Variables|/Game/Blueprints/Components/AC_CharacterAttributes.AC_CharacterAttributes_C|GetHealth _ac_characterattributes) (Variables|/Game/Blueprints/Components/AC_CharacterAttributes.AC_CharacterAttributes_C|GetMaxHealth _ac_characterattributes))))

(fn InitHealthBar
  (bind _aswbp_enemy_healthbar (Utilities|Casting|CastToWBP_EnemyHealthbar (UserInterface|GetWidget (Variables|Default|GetHealthBar))))
  (bind _output_get (Variables|Default|SetHealthBarWidget _aswbp_enemy_healthbar))
  (Default|SetHealthPercent _output_get 1.0)
  (Default|SetDamagePercent _output_get 1.0))

(fn Die
  (|CallParentFunction)
  (CallFunction|DeathStart))

(fn GetLockonLocation
  (return (Transformation|GetSocketLocation (Variables|Character|GetMesh) (Variables|Default|GetTargetLockSocket))))