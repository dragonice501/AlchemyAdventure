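; BP_CharacterBase is the base character Blueprint, providing shared health, damage and attribute queries backed by the ACCharacterAttributes and ACStatusEffects components.
; TakeDamage clamps Health and calls Die at zero, while DamageApplied passes base damage through the status effects component.
; Getters expose alive state, health and stamina ratios, attributes, chain bonus and augmented Might.
; Die, Heal and the status effect HUD functions are empty stubs, and the event graph does nothing.
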(event EventBeginPlay)

(event Collision|EventActorBeginOverlap
  (params (OtherActor :type Actor%20Object%20Reference)))

(event EventTick
  (params (DeltaSeconds :type Float%20%28single-precision%29)))

(fn ConstructionScript)

(fn TakeDamage
  (params (Damage :type Float%20%28double-precision%29))
  (bind _ac_characterattributes (Variables|Default|GetAC_CharacterAttributes))
  (bind _output_get (Variables|/Game/Blueprints/Components/AC_CharacterAttributes.AC_CharacterAttributes_C|SetHealth (Variables|Default|GetAC_CharacterAttributes) (Math|Float|Clamp(Float) (- (Variables|/Game/Blueprints/Components/AC_CharacterAttributes.AC_CharacterAttributes_C|GetHealth _ac_characterattributes) Damage) 0.0 (Variables|/Game/Blueprints/Components/AC_CharacterAttributes.AC_CharacterAttributes_C|GetMaxHealth _ac_characterattributes))))
  (if (<= _output_get 0.0)
    (CallFunction|Die)))

(fn IsAlive
  (return (> (Variables|/Game/Blueprints/Components/AC_CharacterAttributes.AC_CharacterAttributes_C|GetHealth (Variables|Default|GetAC_CharacterAttributes)) 0.0)))

(fn Die)

(fn DamageApplied
  (params (BaseDamage :type Float%20%28double-precision%29))
  (bind _outdamage (Default|EffectDamage (Variables|Default|GetAC_StatusEffects) BaseDamage))
  (return _outdamage))

(fn GetHealthPercent
  (bind _ac_characterattributes (Variables|Default|GetAC_CharacterAttributes))
  (return (Math|Float|SafeDivide (Variables|/Game/Blueprints/Components/AC_CharacterAttributes.AC_CharacterAttributes_C|GetHealth _ac_characterattributes) (Variables|/Game/Blueprints/Components/AC_CharacterAttributes.AC_CharacterAttributes_C|GetMaxHealth _ac_characterattributes))))

(fn GetStaminaPercent
  (bind _ac_characterattributes (Variables|Default|GetAC_CharacterAttributes))
  (return (Math|Float|SafeDivide (Variables|/Game/Blueprints/Components/AC_CharacterAttributes.AC_CharacterAttributes_C|GetStamina _ac_characterattributes) (Variables|/Game/Blueprints/Components/AC_CharacterAttributes.AC_CharacterAttributes_C|GetStaminaMax _ac_characterattributes))))

(fn AddStatusEffectHUD
  (params (StatusEffectWidget :type WBP%20Status%20Effect%20Base%20Class%20Reference) (EffectTime :type Float%20%28double-precision%29) (EffectDuration :type E_EffectDuration%20Enum :default "NewEnumerator0")))

(fn Heal
  (params (Amount :type Integer)))

(fn RemoveStatusEffectHUD
  (params (StatusEffect :type BP%20Status%20Effect%20Base%20Object%20Reference)))

(fn GetAttributes
  (return (Variables|Default|GetAC_CharacterAttributes)))

(fn GetChainBonus
  (return (Variables|/Game/Blueprints/Components/AC_CharacterAttributes.AC_CharacterAttributes_C|GetAttackChainBonus (Variables|Default|GetAC_CharacterAttributes))))

(fn GetMight
  (return (.augmented (Variables|/Game/Blueprints/Components/AC_AttributesBase.AC_AttributesBase_C|GetMightC (Variables|Default|GetAC_CharacterAttributes)))))