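; BP_EnemyDrop is an interactable pickup actor for an item, named as an enemy drop.
; On BeginPlay it spawns a particle system at its location, and SetDropItem assigns the data table row it represents.
; Interact looks up that row and, if found, sends the instigator an AddItem message with the row name and type, then destroys the effect and itself.
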(event EventBeginPlay
  (bind _returnvalue (Niagara|SpawnSystematLocation (Variables|Default|GetSystem%20Template) (Transformation|GetActorLocation)))
  (Variables|Default|SetSpawnedSystem _returnvalue))

(event EventInteract
  (params (Instigator :type Actor%20Object%20Reference))
  (bind _dropitem (Variables|Default|GetDropItem))
  (bind _returnvalue (Utilities|GetDataTableRow (.datatable _dropitem) (.rowname _dropitem))
    (:then
      (Class|BPIInteractable|AddItem(Message) Instigator (Utilities|String|ToString(Name) (.rowname _dropitem)) (Utilities|Struct|BreakS_Item _returnvalue))
      (Components|DestroyComponent (Variables|Default|GetSpawnedSystem))
      (Actor|DestroyActor))))

(fn ConstructionScript
  (|CallParentFunction))

(fn SetDropItem
  (params (Item :type Data%20Table%20Row%20Handle%20Structure))
  (Variables|Default|SetDropItem Item))